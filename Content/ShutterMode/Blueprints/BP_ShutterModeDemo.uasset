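; BP_ShutterModeDemo is a demo Blueprint for the Shutter Mode photo-mode system.
; On BeginPlay it adds the demo HUD, enables the mouse with Game and UI input, and prints the photo directory.
; Thin wrapper functions expose photo mode entry, exit and toggle, filter cycling, wide-open and stopped-down aperture presets, guide toggling and photo capture.
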(event `self.ReceiveBeginPlay`
  (bind _returnvalue (`GameplayStatics.GetPlayerController` 0))
  (bind _returnvalue_2 (`|CreateWidget` "/ShutterMode/ShutterMode/UI/WBP_ShutterModeDemoHUD.WBP_ShutterModeDemoHUD_C" _returnvalue))
  (`UserWidget.AddToViewport` _returnvalue_2 0)
  (set `PlayerController.bShowMouseCursor` true _returnvalue)
  (`WidgetBlueprintLibrary.SetInputMode_GameAndUIEx` _returnvalue null "DoNotLock" false)
  (`KismetSystemLibrary.PrintString` (`ShutterModeSubsystem.GetPhotoDirectory` (`ShutterModeStatics.GetShutterMode`)) false))

(fn `ApertureStoppedDown`
  (`ShutterModeSubsystem.SetAperture` (`ShutterModeStatics.GetShutterMode`) 8.0))

(fn `ApertureWideOpen`
  (`ShutterModeSubsystem.SetAperture` (`ShutterModeStatics.GetShutterMode`) 1.4))

(fn `EnterPhotoMode`
  (`ShutterModeStatics.EnterPhotoMode` null))

(fn `ExitPhotoMode`
  (`ShutterModeStatics.ExitPhotoMode`))

(fn `NextFilter`
  (`ShutterModeStatics.NextFilter`))

(fn `TakePhoto`
  (`ShutterModeStatics.CapturePhoto` 2))

(fn `ToggleGuides`
  (`ShutterModeSubsystem.SetGuidesEnabled` (`ShutterModeStatics.GetShutterMode`) (not (`.bGuides` (break `ShutterModeState` (`ShutterModeStatics.GetState`))))))

(fn `TogglePhotoMode`
  (`ShutterModeStatics.TogglePhotoMode` null))

(fn `UserConstructionScript`)